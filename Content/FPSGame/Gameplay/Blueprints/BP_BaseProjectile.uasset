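; BP_BaseProjectile is a base projectile Blueprint that launches toward the player's camera aim on spawn.
; BeginPlay sets its velocity along the direction from the MainCharacter's weapon mesh to a distant point on the camera's forward axis, without a trace.
; Sphere collision starts disabled and a short timer then enables query and physics collision.
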(event Custom|CustomEvent
  (Collision|SetCollisionEnabled (Variables|Default|GetSphereCollision) "QueryAndPhysics"))

(event EventBeginPlay
  (bind _returnvalue (Game|GetPlayerCameraManager 0))
  (Collision|SetCollisionEnabled (Variables|Default|GetSphereCollision) "NoCollision")
  (Variables|/Script/Engine.MovementComponent|SetVelocity (Variables|Default|GetProjectileComponent) (* 2e+03 (Math|Vector|Normalize (- (+ (* 6e+03 (Transformation|GetActorForwardVector _returnvalue)) (Transformation|GetActorLocation _returnvalue)) (.location (Transformation|GetSocketTransform (Class|ActiveWeaponComponent|GetWeaponMesh (Variables|/Script/FPS.MainCharacter|GetWeaponComponent (.AsMain%20Character (Utilities|Casting|CastToMainCharacter (Game|GetPlayerCharacter 0))))) "None" "RTS_World"))))))
  (|CallParentFunction)
  (Utilities|Time|SetTimerbyEvent (delegate Custom|CustomEvent) 0.02))

(fn ConstructionScript)