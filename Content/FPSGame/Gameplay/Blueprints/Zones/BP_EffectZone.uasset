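; BP_EffectZone is a zone that repeatedly applies a configurable Gameplay Effect to an overlapping actor's Ability System Component.
; Begin overlap opens a Gate and enters it, applying the effect spec with ValueToApply as a SetByCaller magnitude under Message.Effect.Set.
; A Delay of Cooldown re-enters the Gate to repeat the application.
; End overlap of any actor closes the single shared Gate, stopping the loop.
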(event OnComponentBeginOverlap(CollisionComponent)
  (params (OverlappedComponent :type Primitive%20Component%20Object%20Reference) (OtherActor :type Actor%20Object%20Reference) (OtherComp :type Primitive%20Component%20Object%20Reference) (OtherBodyIndex :type Integer) (bFromSweep :type Boolean) (SweepResult :type Hit%20Result%20Structure%20%28by%20ref%29))
  (bind _returnvalue (Ability|GetAbilitySystemComponent OtherActor))
  (Utilities|FlowControl|Sequence
    (:then_0
      (goto _label Open))
    (:then_1
      (Utilities|FlowControl|Gate true :!label _label
        (:Exit
          (bind _returnvalue_2 (Ability|GameplayEffect|AssignTagSetbyCallerMagnitude (GameplayEffects|MakeOutgoingSpec :self _returnvalue :GameplayEffectClass (Variables|Default|GetEffectToApply)) "(TagName=\"Message.Effect.Set\")" (Variables|Default|GetValueToApply)))
          (GameplayEffects|ApplyGameplayEffectSpecToSelf _returnvalue _returnvalue_2)
          (Utilities|FlowControl|Delay (Variables|Default|GetCooldown))
          (goto _label))))))

(event OnComponentEndOverlap(CollisionComponent)
  (params (OverlappedComponent :type Primitive%20Component%20Object%20Reference) (OtherActor :type Actor%20Object%20Reference) (OtherComp :type Primitive%20Component%20Object%20Reference) (OtherBodyIndex :type Integer))
  (Utilities|FlowControl|Gate true) ; enters at Close
)

(event EventBeginPlay)

(fn ConstructionScript)